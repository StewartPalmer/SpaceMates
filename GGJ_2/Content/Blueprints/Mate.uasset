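; Mate is an actor Blueprint that holds helpers for a randomized gameplay sequence, with empty event and construction graphs.
; RandomiseSequence fills the first seven slots of GamePlayStorage with random integers from LevelMin to a fixed upper bound, ignoring its Max input.
; The LoopDelay macro is a stepped for loop that advances only when NextStep fires, allowing delays between iterations, and supports Break.
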(event EventBeginPlay)

(fn ConstructionScript)

(fn RandomiseSequence
  (params (Max :type Integer))
  (for _index (range 0 6)
    (Utilities|Array|SetArrayElem (Variables|Default|GetGame%20Play%20Storage) _index (Math|Random|RandomIntegerinRange (Variables|Default|GetLevel%20Min) 5)))
  (return))