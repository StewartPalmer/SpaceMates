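; TimeGraph is a rhythm-timing Blueprint that scores game time against a fixed-BPM metronome and logs the result to a string array every Tick.
; CalcPlayerScore raises MetronomeGraph's Y to an absolute fifth power, sharpening timing peaks.
; ManageGameTimeline returns the current sequence index only above a score threshold after the first half bar, otherwise -1, and flags sequence end.
; MetronomeGraph's cosine and bar-count math appears unconnected.
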(event EventTick
  (params (DeltaSeconds :type Float%20%28single-precision%29))
  (bind _returnvalue (Utilities|Time|GetGameTimeinSeconds))
  (bind (_score _arrayindex) (CallFunction|ManageGameTimeline _returnvalue 1.2e+02 6))
  (Utilities|Array|Add (Variables|Default|GetstringArray) (Utilities|String|Append "Time " (Utilities|String|ToString(Float) _returnvalue) "         Score: " (Utilities|String|ToString(Float) _score) "         Current Sequence: " (Utilities|String|ToString(Integer) _arrayindex))))

(fn ConstructionScript)

(fn CalcPlayerScore
  (params (time :type Float%20%28single-precision%29) (BPM :type Float%20%28single-precision%29))
  (bind (_y _currentsequence _secondsperbar) (Utilities|MetronomeGraph time BPM))
  (return (Math|Float|Absolute(Float) (Math|Float|Power _y 5.0)) _currentsequence _secondsperbar))

(fn ManageGameTimeline
  (params (time :type Float%20%28single-precision%29) (BPM :type Float%20%28single-precision%29) (sequenceLength :type Integer))
  (bind (_score _currentsequence _secondsperbar) (CallFunction|CalcPlayerScore time BPM))
  (if (or (<= _score 0.3) (< time (/ _secondsperbar 2.0)))
    (return _score -1 (> _currentsequence sequenceLength))
    (else
      (return _score _currentsequence (> _currentsequence sequenceLength)))))