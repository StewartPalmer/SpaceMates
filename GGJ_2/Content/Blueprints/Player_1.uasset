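; Player 1 alien character that plays a Paper2D flipbook dance move on each W, A, S, D or F key press.
; BeginPlay runs Reset_Anim to enable input and hide and rewind the five move flipbooks.
; Five identical per-key macros swap idle for the move, disable input for the flipbook's length, then restore idle and input.
; NewMacro_0 is an unconnected hardcoded version of the Down move.
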(event EventBeginPlay
  (|Reset_Anim (Variables|Default|GetAlien_1_Up) (Variables|Default|GetAlien_1_Down) (Variables|Default|GetAlien_1_Left) (Variables|Default|GetAlien_Right_1) (Variables|Default|GetAlien_1_Final)))

(event EventBeginPlay)

(event Input|KeyboardEvents|F
  (params (Key :type Key%20Structure :default "AnyKey"))
  (:Pressed
    (|F (Variables|Default|GetAlien_1_Final) (Variables|Default|GetAlien_Idle_1))))

(event Input|KeyboardEvents|W
  (params (Key :type Key%20Structure :default "AnyKey"))
  (:Pressed
    (|W (Variables|Default|GetAlien_1_Up) (Variables|Default|GetAlien_Idle_1))))

(event Input|KeyboardEvents|W
  (params (Key :type Key%20Structure :default "AnyKey")))

(event Input|KeyboardEvents|S
  (params (Key :type Key%20Structure :default "AnyKey"))
  (:Pressed
    (|S (Variables|Default|GetAlien_1_Down) (Variables|Default|GetAlien_Idle_1))))

(event Input|KeyboardEvents|A
  (params (Key :type Key%20Structure :default "AnyKey"))
  (:Pressed
    (|A (Variables|Default|GetAlien_1_Left) (Variables|Default|GetAlien_Idle_1))))

(event Input|KeyboardEvents|D
  (params (Key :type Key%20Structure :default "AnyKey"))
  (:Pressed
    (|D (Variables|Default|GetAlien_Right_1) (Variables|Default|GetAlien_Idle_1))))

(fn ConstructionScript)