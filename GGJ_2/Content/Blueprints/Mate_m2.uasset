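; Mate_m2 is a flipbook-animated mate actor that plays one-shot move animations whenever MoveEvent fires.
; The event's Animation value indexes GamePlayStorage to select an M2 idle, directional or crazy flipbook for the AlienRight1 component.
; During playback it hides the Idle component and disables player input, using a Delay of the flipbook's length to restore both afterwards.
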(event Custom|MoveEvent_Event_Copy
  (params (Animation :type Integer))
  (bind _alien_right_1 (Variables|Default|GetAlien_Right_1))
  (bind _idle (Variables|Default|GetIdle))
  (Sprite|SetFlipbook _alien_right_1 (Utilities|Select :Index (Utilities|Array|Get(acopy) (Variables|Default|GetGame%20Play%20Storage) Animation) :Option%200 "/Game/Monster_2/M2_Idle/M2_Idle.M2_Idle" :Option%201 "/Game/Monster_2/M2_Up/M2_Up.M2_Up" :Option%202 "/Game/Monster_2/M2_Down/M2_Down.M2_Down" :Option%203 "/Game/Monster_2/M2_Left/M2_Left.M2_Left" :Option%204 "/Game/Monster_2/M2_Right/M2_right.M2_right" :Option%205 "/Game/Monster_2/M2_Crazy/M2_Crazy.M2_Crazy"))
  (Rendering|SetVisibility _idle false false)
  (Input|DisableInput (Game|GetPlayerController 0))
  (Rendering|SetVisibility _alien_right_1 true false)
  (Audio|Components|Audio|Play _alien_right_1)
  (Utilities|FlowControl|Delay (Class|PaperFlipbookComponent|GetFlipbookLength _alien_right_1))
  (Audio|Components|Audio|Stop _alien_right_1)
  (Components|Timeline|SetPlaybackPosition _alien_right_1 0.0 false)
  (Rendering|SetVisibility _alien_right_1 false false)
  (Input|EnableInput (Game|GetPlayerController 0))
  (Rendering|SetVisibility _idle true false))

(event EventBeginPlay
  (bind _alien_right_1 (Variables|Default|GetAlien_Right_1))
  (Utilities|FlowControl|Sequence
    (:then_0
      (Input|EnableInput (Game|GetPlayerController 0))
      (Components|Timeline|SetPlaybackPosition _alien_right_1 0.0 false)
      (Audio|Components|Audio|Stop _alien_right_1)
      (Rendering|SetVisibility _alien_right_1 false false))
    (:then_1
      (EventDispatchers|BindEventtoMoveEvent (delegate Custom|MoveEvent_Event_Copy)))))

(event EventBeginPlay
  (|CallParentFunction))

(event Collision|EventActorBeginOverlap
  (params (OtherActor :type Actor%20Object%20Reference)))

(event EventTick
  (params (DeltaSeconds :type Float%20%28single-precision%29)))

(fn ConstructionScript
  (|CallParentFunction))