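; Player 2 gamepad Blueprint that turns face-button and trigger presses into directional or "crazy" flipbook animations for an MC character.
; Each input sets a key code, with both triggers together giving the crazy one, and broadcasts it through the KeyPressB dispatcher.
; The bound handler selects the flipbook and calls Play Anim, which hides the idle sprite and disables player controller 1 input until playback ends.
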(event Custom|KeyPress_Event
  (params (Key :type Integer))
  (bind _mc_main (Variables|Default|GetMC_Main))
  (Sprite|SetFlipbook _mc_main (Utilities|Select :Index Key :Option%200 "/Game/Sprites/Main_Character/FlipBooks/MC_Idle.MC_Idle" :Option%201 "/Game/Sprites/Main_Character/FlipBooks/MC_Up.MC_Up" :Option%202 "/Game/Sprites/Main_Character/FlipBooks/MC_Down.MC_Down" :Option%203 "/Game/Sprites/Main_Character/FlipBooks/MC_Left.MC_Left" :Option%204 "/Game/Sprites/Main_Character/FlipBooks/MC_Right.MC_Right" :Option%205 "/Game/Sprites/Main_Character/FlipBooks/MC_Crazy.MC_Crazy"))
  (|PlayAnim _mc_main (Variables|Default|GetMC_Idle)))

(event EventBeginPlay
  (Input|EnableInput (Game|GetPlayerController 1))
  (EventDispatchers|BindEventtoKeyPressB (delegate Custom|KeyPress_Event)))

(event Input|GamepadEvents|GamepadFaceButtonBottom
  (params (Key :type Key%20Structure :default "AnyKey"))
  (:Pressed
    (Variables|Default|SetGamePad_B 1)
    (Default|CallKeyPressB (Variables|Default|GetGamePad_B) :!label _label))
  (:Released
    (Variables|Default|SetGamePad_B 0)
    (goto _label)))

(event Input|GamepadEvents|GamepadFaceButtonLeft
  (params (Key :type Key%20Structure :default "AnyKey"))
  (:Pressed
    (Variables|Default|SetGamePad_B 2)
    (Default|CallKeyPressB (Variables|Default|GetGamePad_B) :!label _label))
  (:Released
    (Variables|Default|SetGamePad_B 0)
    (goto _label)))

(event Input|GamepadEvents|GamepadFaceButtonRight
  (params (Key :type Key%20Structure :default "AnyKey"))
  (:Pressed
    (Variables|Default|SetGamePad_B 3)
    (Default|CallKeyPressB (Variables|Default|GetGamePad_B) :!label _label))
  (:Released
    (Variables|Default|SetGamePad_B 0)
    (goto _label)))

(event Input|GamepadEvents|GamepadFaceButtonTop
  (params (Key :type Key%20Structure :default "AnyKey"))
  (:Pressed
    (Variables|Default|SetGamePad_B 4)
    (Default|CallKeyPressB (Variables|Default|GetGamePad_B) :!label _label))
  (:Released
    (Variables|Default|SetGamePad_B 0)
    (goto _label)))

(event Input|GamepadEvents|GamepadLeftTrigger
  (params (Key :type Key%20Structure :default "AnyKey"))
  (:Pressed
    (bind _output_get (Variables|Default|SetGP_LT true))
    (if (and _output_get (stale Input|GamepadEvents|GamepadRightTrigger _output_get))
      (Utilities|FlowControl|Sequence
        (:then_0
          (Variables|Default|SetGP_LT false))
        (:then_1
          (Variables|Default|SetGP_RT false)))
      (Variables|Default|SetGamePad_B 5)
      (else
        (Variables|Default|SetGamePad_B 0)))
    (Default|CallKeyPressB (Variables|Default|GetGamePad_B)))
  (:Released
    (Variables|Default|SetGP_LT false)))

(event Input|GamepadEvents|GamepadRightTrigger
  (params (Key :type Key%20Structure :default "AnyKey"))
  (:Pressed
    (bind _output_get (Variables|Default|SetGP_RT true))
    (if (and (stale Input|GamepadEvents|GamepadLeftTrigger _output_get) _output_get)
      (Utilities|FlowControl|Sequence
        (:then_0
          (Variables|Default|SetGP_LT false))
        (:then_1
          (Variables|Default|SetGP_RT false)))
      (Variables|Default|SetGamePad_B 5)
      (else
        (Variables|Default|SetGamePad_B 0)))
    (Default|CallKeyPressB (Variables|Default|GetGamePad_B)))
  (:Released
    (Variables|Default|SetGP_RT false)))

(fn ConstructionScript)